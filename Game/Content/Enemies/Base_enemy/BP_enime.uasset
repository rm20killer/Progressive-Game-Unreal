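; BP_enime is a base enemy actor with health and a targeting marker.
; Health starts at MaxHealth on BeginPlay, and TakeDamage subtracts damage, destroys the actor when health drops below 1, and returns whether it died.
; IsTargeted shows or hides the marker widget and its children, and GetTracker exposes the BPTracker reference to callers.
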(event `self.ReceiveBeginPlay`
  (set `self.Health` (`self.MaxHealth`)))

(fn `GetTracker`
  (returns (BP_Tracker :type "/Game/Attack_particles/BP_Tracker Object Reference"))
  (return (`self.BP_Tracker`)))

(fn `IsTargeted`
  (params (Target :type Boolean))
  ;[1 1 1] Make marker visible or not
  (`SceneComponent.SetVisibility` (`self.Widget`) Target true))

(fn `TakeDamage`
  (params (Damage :type Integer))
  (returns (Dead :type Boolean))
  (bind _output_get (set `self.Health` (- (`self.Health`) Damage)))
  (bind _returnvalue (< _output_get 1))
  (if _returnvalue
    (`self.K2_DestroyActor`))
  (return _returnvalue))

(fn `UserConstructionScript`)