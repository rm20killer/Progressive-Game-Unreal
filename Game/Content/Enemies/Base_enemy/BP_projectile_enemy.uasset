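; Projectile actor fired by enemies that damages the player character on contact.
; It expires after a short lifespan set on BeginPlay.
; Overlapping ThirdPersonCharacter calls its TakeDamage, spawns an impact particle and destroys the projectile; other overlaps are ignored.
; Blocking hits on the sphere collider spawn the same effect and destroy it without dealing damage.
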(event `self.ReceiveBeginPlay`
  (`self.SetLifeSpan` 5.0))

(event `self.Sphere.OnComponentBeginOverlap`
  (params (OverlappedComponent :type "PrimitiveComponent Object Reference") (OtherActor :type "Actor Object Reference") (OtherComp :type "PrimitiveComponent Object Reference") (OtherBodyIndex :type Integer) (bFromSweep :type Boolean) (SweepResult :type "HitResult Structure (by ref)"))
  (bind _asthird_person_character (cast `/Game/Agame/Player/Blueprints/ThirdPersonCharacter` OtherActor))
  (`/Game/Agame/Player/Blueprints/ThirdPersonCharacter.Take Damage` _asthird_person_character 5)
  (`GameplayStatics.SpawnEmitterAtLocation` "/Game/Enemies/Base_enemy/p_impact_enemy.p_impact_enemy" (`.Location` (`GameplayStatics.BreakHitResult` SweepResult)))
  (`self.K2_DestroyActor`))

(event `self.Sphere.OnComponentHit`
  (params (HitComponent :type "PrimitiveComponent Object Reference") (OtherActor :type "Actor Object Reference") (OtherComp :type "PrimitiveComponent Object Reference") (NormalImpulse :type "Vector Structure") (Hit :type "HitResult Structure (by ref)"))
  (`GameplayStatics.SpawnEmitterAtLocation` "/Game/Enemies/Base_enemy/p_impact_enemy.p_impact_enemy" (`.Location` (`GameplayStatics.BreakHitResult` Hit)))
  (`self.K2_DestroyActor`))

(fn `UserConstructionScript`)