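; BP_Fireball is a player attack that launches fireballs at nearby enemies.
; Its Fire function loops over BP_enime actors overlapping EnemyFinder, spawning another BP_Fireball at the player pawn, rotated toward each one.
; Each spawn gets a runtime-added projectile movement component, with its homing target set from the enemy's GetParentComponent result.
; Fire also calls the parent implementation, and its Target input is unused.
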(fn `Fire`
  (params (Target :type "Actor Object Reference"))
  (locals (`Homing Target` :type "SceneComponent Object Reference"))
  (bind _returnvalue (`SceneComponent.K2_GetComponentLocation` (`Actor.RootComponent` (`GameplayStatics.GetPlayerPawn` 0))))
  (for _array_element (`PrimitiveComponent.GetOverlappingActors` (`self.EnemyFinder`) "/Game/Enemies/Base_enemy/BP_enime.BP_enime_C")
    (bind _asbp_enime (cast `/Game/Enemies/Base_enemy/BP_enime` _array_element))
    (bind _returnvalue_2 (`|SpawnActorFromClass` "BP_Fireball_C" (`KismetMathLibrary.MakeTransform` _returnvalue (`KismetMathLibrary.FindLookAtRotation` _returnvalue (`SceneComponent.K2_GetComponentLocation` (`Actor.RootComponent` _array_element)))) "AlwaysSpawn" "OverrideRootScale" null null))
    (bind _returnvalue_3 (`AddComponent|NODE_AddProjectileMovementComponent-0` :`self` _returnvalue_2))
    (set `ProjectileMovementComponent.HomingTargetComponent` (`self.GetParentComponent` _asbp_enime) _returnvalue_3))
  (`parent.Fire` null))

(fn `UserConstructionScript`
  (`parent.UserConstructionScript`))