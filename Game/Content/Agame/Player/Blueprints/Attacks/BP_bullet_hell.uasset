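; Player attack that fires a radial bullet-hell burst of BP_projectile actors around the player.
; Overrides Fire, looping over BulletAmmot to spawn projectiles at the player pawn's location, with yaw steps dividing 360 degrees, offset by the camera's yaw.
; Pitch is zeroed to keep the ring level, though camera roll is kept.
; It then plays the magic attack sound and calls the parent Fire; the Target input is unused.
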(fn `Fire`
  (params (Target :type "Actor Object Reference"))
  (locals (BulletAmmot :type Integer :default 25))
  (bind _bulletammot (`local.BulletAmmot`))
  (bind (_returnvalue_location _returnvalue_rotation) (`KismetMathLibrary.BreakTransform` (`SceneComponent.K2_GetComponentToWorld` (`self.Camera`))))
  (bind _returnvalue_location_2 (`KismetMathLibrary.BreakTransform` (`SceneComponent.K2_GetComponentToWorld` (`Actor.RootComponent` (`GameplayStatics.GetPlayerPawn` 0)))))
  (for _index (range (+ _bulletammot 1))
    (`|SpawnActorFromClass` "/Game/Attack_particles/BP_projectile.BP_projectile_C" (`KismetMathLibrary.MakeTransform` _returnvalue_location_2 (`KismetMathLibrary.MakeRotator` (.roll _returnvalue_rotation) 0.0 (+ (* _index (/ 360.0 (`KismetMathLibrary.Conv_IntToDouble` _bulletammot))) (.yaw _returnvalue_rotation)))) "Undefined" "OverrideRootScale" null null))
  (`GameplayStatics.PlaySoundAtLocation` "/Game/Audio/Magic_attack.Magic_attack" _returnvalue_location_2 (struct) 1.0 1.0 0.0 null null null)
  (`parent.Fire` null))

(fn `UserConstructionScript`
  (`parent.UserConstructionScript`))