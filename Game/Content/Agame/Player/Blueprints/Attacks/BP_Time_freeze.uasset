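; Time-freeze attack for the player that toggles slow motion each time Fire is called.
; Fire lowers global time dilation while raising custom dilation on the player pawn and all BP_base_attack actors to compensate, then restores all on the next call.
; Activation costs ManaUsage, and Tick keeps draining the character's mana through a Delay while frozen, calling Fire to end the effect once mana runs out.
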(event `self.ReceiveTick`
  (params (DeltaSeconds :type "Float (single-precision)"))
  (if (`self.IsFreeze`)
    (`KismetSystemLibrary.Delay` 0.1)
    (bind _asthird_person_character (cast `/Game/Agame/Player/Blueprints/ThirdPersonCharacter` (`GameplayStatics.GetPlayerPawn` 0)))
    (`/Game/Agame/Player/Blueprints/ThirdPersonCharacter.ManaUsed` _asthird_person_character 5)
    (if (<= (`/Game/Agame/Player/Blueprints/ThirdPersonCharacter.Mana` _asthird_person_character) 0)
      (`self.Fire` null)
      (`parent.ReceiveTick` DeltaSeconds :!label _label))
    (else
      (goto _label))))

(fn `Fire`
  (params (Target :type "Actor Object Reference"))
  (bind _returnvalue (`GameplayStatics.GetPlayerPawn` 0))
  (if (`self.IsFreeze`)
    ;[1 1 1] Time normal
    (`GameplayStatics.SetGlobalTimeDilation` 1.0)
    (bind _outactors (`GameplayStatics.GetAllActorsOfClass` "/Game/Agame/Player/Blueprints/Attacks/BP_base_attack.BP_base_attack_C"))
    (for _array_element _outactors
      (set `Actor.CustomTimeDilation` 1.0 _array_element))
    (set `Actor.CustomTimeDilation` 1.0 _returnvalue)
    (set `self.IsFreeze` false)
    (else
      ;[1 1 1] Time slow down
      (`GameplayStatics.SetGlobalTimeDilation` 0.1)
      (bind _outactors_2 (`GameplayStatics.GetAllActorsOfClass` "/Game/Agame/Player/Blueprints/Attacks/BP_base_attack.BP_base_attack_C"))
      (for _array_element_2 _outactors_2
        (set `Actor.CustomTimeDilation` 10.0 _array_element_2))
      (set `Actor.CustomTimeDilation` 10.0 _returnvalue)
      (set `self.IsFreeze` true)
      (bind _asthird_person_character (cast `/Game/Agame/Player/Blueprints/ThirdPersonCharacter` _returnvalue))
      (`/Game/Agame/Player/Blueprints/ThirdPersonCharacter.ManaUsed` _asthird_person_character (`self.ManaUsage`))))
  (`parent.Fire` null))

(fn `UserConstructionScript`
  (`parent.UserConstructionScript`))