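; BP_RainAttack is a player attack that rains sky strikes down on nearby enemies.
; Fire ignores its Target input and spawns a scaled-up BP_sky_attack above every BP_enime overlapping EnemyFinder, then calls the parent Fire.
; ManaUsed is called on the ThirdPersonCharacter inside the loop, so mana is charged once per enemy hit by a spawn rather than once per cast.
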(fn `Fire`
  (params (Target :type "Actor Object Reference"))
  (for _array_element (`PrimitiveComponent.GetOverlappingActors` (`self.EnemyFinder`) "/Game/Enemies/Base_enemy/BP_enime.BP_enime_C")
    (bind (_returnvalue_x _returnvalue_y _returnvalue_z) (`KismetMathLibrary.BreakVector` (`self.K2_GetActorLocation` _array_element)))
    (`|SpawnActorFromClass` "/Game/Attack_particles/BP_sky_attack.BP_sky_attack_C" (`KismetMathLibrary.MakeTransform` (`KismetMathLibrary.MakeVector` _returnvalue_x _returnvalue_y (+ _returnvalue_z 500.0)) (struct) (5.0 5.0 5.0)) "Undefined" "OverrideRootScale" null null)
    (bind _asthird_person_character (cast `/Game/Agame/Player/Blueprints/ThirdPersonCharacter` (`GameplayStatics.GetPlayerPawn` 0)))
    (`/Game/Agame/Player/Blueprints/ThirdPersonCharacter.ManaUsed` _asthird_person_character (`self.ManaUsage`)))
  (`parent.Fire` null))

(fn `UserConstructionScript`
  (`parent.UserConstructionScript`))