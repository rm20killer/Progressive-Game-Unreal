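; Magic attack Blueprint that overrides its parent's Fire to launch a BP_projectile from the player's position.
; With a valid target, the projectile is aimed at it by look-at rotation and always spawns regardless of collision.
; Without one, it takes the Camera's rotation and leaves collision handling undefined.
; Both paths then call the parent Fire; the event graph adds no logic of its own.
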(event `self.ReceiveTick`
  (params (DeltaSeconds :type "Float (single-precision)"))
  (`parent.ReceiveTick` DeltaSeconds))

(fn `Fire`
  (params (Target :type "Actor Object Reference"))
  (bind _rootcomponent (`Actor.RootComponent` (`GameplayStatics.GetPlayerPawn` 0)))
  (bind _returnvalue (`SceneComponent.K2_GetComponentLocation` _rootcomponent))
  (bind (_returnvalue_location _returnvalue_rotation) (`KismetMathLibrary.BreakTransform` (`SceneComponent.K2_GetComponentToWorld` (`self.Camera`))))
  (bind _returnvalue_location_2 (`KismetMathLibrary.BreakTransform` (`SceneComponent.K2_GetComponentToWorld` _rootcomponent)))
  (if (`KismetSystemLibrary.IsValid` Target)
    (`|SpawnActorFromClass` "/Game/Attack_particles/BP_projectile.BP_projectile_C" (`KismetMathLibrary.MakeTransform` _returnvalue (`KismetMathLibrary.FindLookAtRotation` _returnvalue (`SceneComponent.K2_GetComponentLocation` (`Actor.RootComponent` Target)))) "AlwaysSpawn" "OverrideRootScale" null null)
    (else
      (`|SpawnActorFromClass` "/Game/Attack_particles/BP_projectile.BP_projectile_C" (`KismetMathLibrary.MakeTransform` _returnvalue_location_2 _returnvalue_rotation) "Undefined" "OverrideRootScale" null null)))
  (`parent.Fire` null))

(fn `UserConstructionScript`
  (`parent.UserConstructionScript`))