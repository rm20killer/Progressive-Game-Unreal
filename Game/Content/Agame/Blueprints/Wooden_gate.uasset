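; Wooden gate Blueprint that moves its Sphere component when a ThirdPersonCharacter enters the Box trigger and returns it on exit.
; Timeline_1 plays and reverses on overlap, lerping the relative location from zero to RelativeMotion.
; A separate Move event, not called here, calls SetNewTime on Timeline_0, whose update flips MoveDown each tick to alternate lerp direction.
; BeginPlay caches the Box location in StartLocation, which is otherwise unused.
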(event `self.ReceiveBeginPlay`
  (set `self.StartLocation` (`SceneComponent.K2_GetComponentLocation` (`self.Box`))))

(event `self.Box.OnComponentBeginOverlap`
  (params (OverlappedComponent :type "PrimitiveComponent Object Reference") (OtherActor :type "Actor Object Reference") (OtherComp :type "PrimitiveComponent Object Reference") (OtherBodyIndex :type Integer) (bFromSweep :type Boolean) (SweepResult :type "HitResult Structure (by ref)"))
  (cast `/Game/Agame/Player/Blueprints/ThirdPersonCharacter` OtherActor)
  (bind (_direction _newtrack_1) (`Timeline|Timeline_1` :!label _label)
    (:`Update`
      (`SceneComponent.K2_SetRelativeLocation` (`self.Sphere`) (`KismetMathLibrary.VLerp` (0.0 0.0 0.0) (`self.RelativeMotion`) _newtrack_1) false false))))

(event `self.Box.OnComponentEndOverlap`
  (params (OverlappedComponent :type "PrimitiveComponent Object Reference") (OtherActor :type "Actor Object Reference") (OtherComp :type "PrimitiveComponent Object Reference") (OtherBodyIndex :type Integer))
  (cast `/Game/Agame/Player/Blueprints/ThirdPersonCharacter` OtherActor)
  (goto _label :!via `Reverse`))

(event `Move`
  (bind _relativemotion (`self.RelativeMotion`))
  (bind _sphere (`self.Sphere`))
  (bind (_direction _newtrack_1) (`Timeline|Timeline_0` :!via `SetNewTime`)
    (:`Update`
      (if (`self.MoveDown`)
        (`SceneComponent.K2_SetRelativeLocation` _sphere (`KismetMathLibrary.VLerp` (0.0 0.0 0.0) _relativemotion _newtrack_1) false false)
        (set `self.MoveDown` false)
        (else
          (`SceneComponent.K2_SetRelativeLocation` _sphere (`KismetMathLibrary.VLerp` _relativemotion (0.0 0.0 0.0) _newtrack_1) false false)
          (set `self.MoveDown` true))))))

(fn `UserConstructionScript`)