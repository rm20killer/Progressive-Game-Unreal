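; BP_Exit is a level exit trigger that reacts when the ThirdPersonCharacter overlaps its Box.
; It finishes the level through BP_GameInstace when CoinsToExit is at least CoinCollectedInRound, as the comparison is written.
; On success it shows WBP_YouWIn with cursor and Game-and-UI input, leaving the game unpaused.
; Otherwise it sets the player character's TipsToShow to a "Not enough Coins" message.
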(event `self.Box.OnComponentBeginOverlap`
  (params (OverlappedComponent :type "PrimitiveComponent Object Reference") (OtherActor :type "Actor Object Reference") (OtherComp :type "PrimitiveComponent Object Reference") (OtherBodyIndex :type Integer) (bFromSweep :type Boolean) (SweepResult :type "HitResult Structure (by ref)"))
  (bind _returnvalue (`GameplayStatics.GetPlayerController` 0))
  (cast `/Game/Agame/Player/Blueprints/ThirdPersonCharacter` OtherActor)
  (bind _asbp_game_instace (cast `/Game/Agame/Blueprints/BP_GameInstace` (`GameplayStatics.GetGameInstance`)))
  (if (>= (`/Game/Agame/Blueprints/BP_GameInstace.CoinsToExit` _asbp_game_instace) (`/Game/Agame/Blueprints/BP_GameInstace.CoinCollectedInRound` _asbp_game_instace))
    (`/Game/Agame/Blueprints/BP_GameInstace.LevelFinished` _asbp_game_instace)
    (bind _returnvalue_2 (`|CreateWidget` "/Game/UI/WBP_YouWIn.WBP_YouWIn_C"))
    (`UserWidget.AddToViewport` _returnvalue_2 0)
    (`GameplayStatics.SetGamePaused` false)
    (set `PlayerController.bShowMouseCursor` true _returnvalue)
    (`WidgetBlueprintLibrary.SetInputMode_GameAndUIEx` _returnvalue _returnvalue_2 "LockInFullscreen")
    (else
      (bind _asthird_person_character (cast `/Game/Agame/Player/Blueprints/ThirdPersonCharacter` (`GameplayStatics.GetPlayerPawn` 0)))
      (set `/Game/Agame/Player/Blueprints/ThirdPersonCharacter.TipsToShow` "Not enough Coins" _asthird_person_character))))

(fn `UserConstructionScript`)