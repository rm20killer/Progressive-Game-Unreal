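; BP_BigBall_projectile is a big-ball attack projectile with a five-second lifespan that damages enemies on sphere overlap.
; Overlaps with the player character, BP_projectile and other big balls are ignored.
; An enemy hit calls TakeDamage and, if that returns false, adds a world-backward force to the enemy's movement.
; Enemy hits and any other overlap then fire a RadialForce impulse and destroy the ball.
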(event `self.Sphere.OnComponentBeginOverlap`
  (params (OverlappedComponent :type "PrimitiveComponent Object Reference") (OtherActor :type "Actor Object Reference") (OtherComp :type "PrimitiveComponent Object Reference") (OtherBodyIndex :type Integer) (bFromSweep :type Boolean) (SweepResult :type "HitResult Structure (by ref)"))
  (cast `/Game/Agame/Player/Blueprints/ThirdPersonCharacter` OtherActor
    (:`CastFailed`
      (bind _asbp_enime (cast `/Game/Enemies/Base_enemy/BP_enime` OtherActor)
        (:`then`
          (`KismetSystemLibrary.PrintString` (`KismetStringLibrary.BuildString_Object` "Damaged to " "" _asbp_enime (`KismetSystemLibrary.GetDisplayName` OtherActor)))
          (bind _dead (`/Game/Enemies/Base_enemy/BP_enime.TakeDamage` _asbp_enime (`self.Damage`)))
          (if (not _dead)
            (`CharacterMovementComponent.AddForce` (`Character.CharacterMovement` _asbp_enime) (* (`KismetMathLibrary.Vector_Backward`) 100.0))))
        (:`CastFailed`
          (cast `/Game/Attack_particles/BP_projectile` OtherActor
            (:`CastFailed`
              (cast `/Game/Attack_particles/BP_BigBall_projectile` OtherActor
                (:`CastFailed`
                  _))))))
      (`RadialForceComponent.FireImpulse` (`self.RadialForce`))
      (`self.K2_DestroyActor`))))

(event `self.ReceiveBeginPlay`
  (`self.SetLifeSpan` 5.0))

(fn `UserConstructionScript`)