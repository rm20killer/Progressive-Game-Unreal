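; BP_sky_attack is a short-lived spell actor that drops a volley of BP_BigBall_projectile actors pointing straight down.
; On BeginPlay it calls Fire, then sets a two-second lifespan on itself.
; Fire loops to spawn the projectiles at random horizontal and vertical offsets around the PAttackSpell component's world location, ignoring collision.
; An EnemyFinder reference is present but unused.
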(event `self.ReceiveBeginPlay`
  (`self.Fire`)
  (`self.SetLifeSpan` 2.0))

(fn `Fire`
  (bind _returnvalue (`KismetMathLibrary.RandomFloatInRange` -100.0 100.0))
  (for _index (range 11)
    (`|SpawnActorFromClass` "/Game/Attack_particles/BP_BigBall_projectile.BP_BigBall_projectile_C" (`KismetMathLibrary.MakeTransform` (`KismetMathLibrary.MakeVector` (+ _returnvalue (.x (`SceneComponent.K2_GetComponentLocation` (`self.p_attack_spell`)))) (+ _returnvalue (.y (`SceneComponent.K2_GetComponentLocation` (`self.p_attack_spell`)))) (+ (.z (`SceneComponent.K2_GetComponentLocation` (`self.p_attack_spell`))) (`KismetMathLibrary.RandomFloatInRange` -50.0 350.0))) (`KismetMathLibrary.MakeRotator` 0.0 -90.0)) "AlwaysSpawn" "OverrideRootScale" null null)))

(fn `UserConstructionScript`)