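; Healing shrine actor that periodically heals a ThirdPersonCharacter standing inside its Box trigger.
; Box overlap events set a Healing flag and store the entering character as Player, then clear the flag on exit.
; A looping one-second timer, started on BeginPlay, checks the flag and calls the stored character's Heal with HealAmount.
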(event `self.ReceiveBeginPlay`
  ;[1 1 1] call heal event every 1 sec
  (`KismetSystemLibrary.K2_SetTimer` null "Heal" 1.0 true))

(event `self.Box.OnComponentBeginOverlap`
  (params (OverlappedComponent :type "PrimitiveComponent Object Reference") (OtherActor :type "Actor Object Reference") (OtherComp :type "PrimitiveComponent Object Reference") (OtherBodyIndex :type Integer) (bFromSweep :type Boolean) (SweepResult :type "HitResult Structure (by ref)"))
  ;[1 1 1] Heal while in
  (cast `/Game/Agame/Player/Blueprints/ThirdPersonCharacter` OtherActor)
  (set `self.Healing` true)
  (set `self.Player` OtherActor))

(event `self.Box.OnComponentEndOverlap`
  (params (OverlappedComponent :type "PrimitiveComponent Object Reference") (OtherActor :type "Actor Object Reference") (OtherComp :type "PrimitiveComponent Object Reference") (OtherBodyIndex :type Integer))
  ;[1 1 1] Dont heal once out
  (cast `/Game/Agame/Player/Blueprints/ThirdPersonCharacter` OtherActor)
  (set `self.Healing` false))

(event `Heal`
  ;[1 1 1] Heal event
  (if (`self.Healing`)
    (bind _asthird_person_character (cast `/Game/Agame/Player/Blueprints/ThirdPersonCharacter` (`self.Player`)))
    (`/Game/Agame/Player/Blueprints/ThirdPersonCharacter.Heal` _asthird_person_character (`self.HealAmount`))))

(fn `UserConstructionScript`)