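; Game instance that tracks coins collected, elapsed time and records for level runs.
; CoinCollected and OneSecoundPassed each increment their counter by one.
; LevelFinished raises HighestCoinCount to the round's coins when matched or beaten, but sets HighestTime to zero, rather than TimeToComplete, when the time is at or below it.
; Neither running counter is reset here.
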(fn `CoinCollected`
  (set `self.CoinCollectedInRound` (+ (`self.CoinCollectedInRound`) 1)))

(fn `LevelFinished`
  (if (<= (`self.TimeToComplete`) (`self.HighestTime`))
    (set `self.HighestTime` 0))
  (if (>= (`self.CoinCollectedInRound`) (`self.HighestCoinCount`))
    (set `self.HighestCoinCount` (`self.CoinCollectedInRound`))))

(fn `OneSecoundPassed`
  (set `self.TimeToComplete` (+ (`self.TimeToComplete`) 1)))