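; Base player attack Blueprint with cooldown, mana cost and nearest-enemy targeting, with an empty Fire function as the override point.
; FireEvent picks the closest overlapping BP_enime, updates its targeted flag, then calls Fire once the Tick-driven cooldown expires.
; Firing resets the cooldown and charges ThirdPersonCharacter mana unless DontTakeManaOnFire is set.
; CanFire reports mana and cooldown readiness, but FireEvent checks only cooldown itself.
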(event `self.ReceiveBeginPlay`
  (set `self.CooldownTimer` (`self.Cooldown`)))

(event `self.ReceiveTick`
  (params (DeltaSeconds :type "Float (single-precision)"))
  (set `self.CooldownTimer` (- (`self.CooldownTimer`) DeltaSeconds)))

(event `FireEvent`
  (`self.FindCloestEnemy`)
  (if (<= (`self.CooldownTimer`) 0.0)
    (`self.Fire` (`self.CurrentTarget`))
    (if (not (`self.DontTakeManaOnFire`))
      (bind _asthird_person_character (cast `/Game/Agame/Player/Blueprints/ThirdPersonCharacter` (`GameplayStatics.GetPlayerPawn` 0)))
      (`/Game/Agame/Player/Blueprints/ThirdPersonCharacter.ManaUsed` _asthird_person_character (`self.ManaUsage`)))
    (set `self.CooldownTimer` (`self.Cooldown`))))

(event `FindCloestEnemy`
  (bind _overlappingactors (`self.GetOverlappingActors` "/Game/Enemies/Base_enemy/BP_enime.BP_enime_C"))
  (bind _currenttarget (`self.CurrentTarget`))
  ;[1 1 1] Get cloest enemy
  (if (>= (`KismetArrayLibrary.Array_Length` _overlappingactors) 1)
    (set `self.CurrentTarget` (`|GetArrayItem` _overlappingactors))
    (for _array_element _overlappingactors
      (if (<= (`self.GetDistanceTo` _array_element self) (`self.GetDistanceTo` _currenttarget self))
        (set `self.CurrentTarget` _array_element)
        (else
          (bind _asbp_enime (cast `/Game/Enemies/Base_enemy/BP_enime` _array_element))
          (`/Game/Enemies/Base_enemy/BP_enime.IsTargeted` _asbp_enime false))))
    (if (`self.IsActorBeingDestroyed` _currenttarget)
      (set `self.CurrentTarget` null)
      (else
        (bind _asbp_enime_2 (cast `/Game/Enemies/Base_enemy/BP_enime` _currenttarget))
        (`/Game/Enemies/Base_enemy/BP_enime.IsTargeted` _asbp_enime_2 true)))
    (else
      (bind _asbp_enime_3 (cast `/Game/Enemies/Base_enemy/BP_enime` (`self.CurrentTarget`)))
      (`/Game/Enemies/Base_enemy/BP_enime.IsTargeted` _asbp_enime_3 false)
      (set `self.CurrentTarget` null))))

(fn `CanFire`
  (returns (CanUse :type Boolean))
  (bind _asthird_person_character (cast `/Game/Agame/Player/Blueprints/ThirdPersonCharacter` (`GameplayStatics.GetPlayerPawn` 0)))
  (if (<= (`/Game/Agame/Player/Blueprints/ThirdPersonCharacter.Mana` _asthird_person_character) (`self.ManaUsage`))
    _
    (elif (<= (`self.CooldownTimer`) 0.0)
      (return true)
      (else
        _)))
  (return false))

(fn `Fire`
  (params (Target :type "Actor Object Reference"))
  (return))

(fn `UserConstructionScript`)