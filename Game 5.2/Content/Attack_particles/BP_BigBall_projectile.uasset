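; BP_BigBall_projectile is a projectile that damages BP_enime actors and expires after five seconds.
; Sphere overlaps ignore ThirdPersonCharacter and both projectile classes, while anything else fires a RadialForce impulse.
; Enemies also get an impact emitter and Damage, destroying the ball only if TakeDamage returns true; other overlaps destroy it directly.
; Blocking hits spawn the emitter and destroy it without an impulse.
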(event `self.Sphere.OnComponentBeginOverlap`
  (params (OverlappedComponent :type "PrimitiveComponent Object Reference") (OtherActor :type "Actor Object Reference") (OtherComp :type "PrimitiveComponent Object Reference") (OtherBodyIndex :type Integer) (bFromSweep :type Boolean) (SweepResult :type "HitResult Structure (by ref)"))
  (cast `/Game/Agame/Player/Blueprints/ThirdPersonCharacter` OtherActor
    (:`CastFailed`
      (bind _asbp_enime (cast `/Game/Enemies/Base_enemy/BP_enime` OtherActor)
        (:`then`
          (`GameplayStatics.SpawnEmitterAtLocation` "/Game/Attack_particles/SkyStrike/Skyattack/p_impact_sky.p_impact_sky" (`.Location` (`GameplayStatics.BreakHitResult` SweepResult)))
          (`RadialForceComponent.FireImpulse` (`self.RadialForce`))
          (bind _dead (`/Game/Enemies/Base_enemy/BP_enime.TakeDamage` _asbp_enime (`self.Damage`)))
          (if _dead
            (`self.K2_DestroyActor` :!label _label)))
        (:`CastFailed`
          (cast `/Game/Attack_particles/BP_projectile` OtherActor
            (:`CastFailed`
              (cast `/Game/Attack_particles/BP_BigBall_projectile` OtherActor
                (:`CastFailed`
                  (`RadialForceComponent.FireImpulse` (`self.RadialForce`))
                  (goto _label))))))))))

(event `self.ReceiveBeginPlay`
  (`self.SetLifeSpan` 5.0))

(event `self.Sphere.OnComponentHit`
  (params (HitComponent :type "PrimitiveComponent Object Reference") (OtherActor :type "Actor Object Reference") (OtherComp :type "PrimitiveComponent Object Reference") (NormalImpulse :type "Vector Structure") (Hit :type "HitResult Structure (by ref)"))
  (`GameplayStatics.SpawnEmitterAtLocation` "/Game/Attack_particles/SkyStrike/Skyattack/p_impact_sky.p_impact_sky" (`.Location` (`GameplayStatics.BreakHitResult` Hit)) (struct))
  (`self.K2_DestroyActor`))

(fn `UserConstructionScript`)