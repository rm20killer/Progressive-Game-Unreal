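; Base enemy Blueprint that holds health, shows a target marker and can be destroyed by damage.
; Health starts at MaxHealth, and TakeDamage subtracts from it, plays an explosion sound at the mesh and destroys the actor below 1, returning whether it died.
; IsTargeted toggles the marker widget's visibility, and GetTracker exposes its BPTracker to callers.
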(event `self.ReceiveBeginPlay`
  (set `self.Health` (`self.MaxHealth`)))

(fn `GetTracker`
  (returns (BP_Tracker :type "/Game/Attack_particles/BP_Tracker Object Reference"))
  (return (`self.BP_Tracker`)))

(fn `IsTargeted`
  (params (Target :type Boolean))
  ;[1 1 1] Make marker visible or not
  (`SceneComponent.SetVisibility` (`self.Widget`) Target true))

(fn `TakeDamage`
  (params (Damage :type Integer))
  (returns (Dead :type Boolean))
  (bind _output_get (set `self.Health` (- (`self.Health`) Damage)))
  (bind _returnvalue (< _output_get 1))
  (if _returnvalue
    (`GameplayStatics.PlaySoundAtLocation` "/Game/StarterContent/Audio/Explosion01.Explosion01" (`SceneComponent.K2_GetComponentLocation` (`self.Mesh`)) (struct) 0.2 1.0 0.0 null null self)
    (`self.K2_DestroyActor`))
  (return _returnvalue))

(fn `UserConstructionScript`)